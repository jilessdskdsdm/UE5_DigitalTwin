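; BP_MainMenuController is an input-enabled actor that handles main-menu house-type display and audio.
; StartShow toggles tagged actors by house type name, playing a timeline that drives the "进度" (progress) scalar material parameter on show and stopping it on hide.
; It pauses background music on BeginPlay, exposes SetBGM to pause or resume it, and PlayOthersMusic swaps and plays sounds on a separate audio component.
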(event `StartShow`
  (params (HouseTypeName :type Name) (bIsShow :type Boolean))
  (`FunctionLibrary.SetTagActorShow` HouseTypeName bIsShow)
  (if bIsShow
    (bind (_direction `_新建轨道_2`) (`Timeline|时间轴` :!via `PlayFromStart` :!label _label)
      (:`Update`
        (`KismetMaterialLibrary.SetScalarParameterValue` null "进度" `_新建轨道_2`)))
    (else
      (goto _label :!via `Stop`))))

(event `self.ReceiveBeginPlay`
  (`self.EnableInput` (`GameplayStatics.GetPlayerController` 0))
  (`/DigitalTwin/Data/FL_FunctionLibrary.PauseBackgroundMusic` true))

(event `SetBGM`
  (params (bPause :type Boolean))
  (`AudioComponent.SetPaused` (`self.BackgroundMusic`) bPause))

(fn `PlayOthersMusic`
  (params (NewSound :type "SoundBase Object Reference"))
  (bind _othersmusic (`self.OthersMusic`))
  (`AudioComponent.SetSound` _othersmusic NewSound)
  (`AudioComponent.Play` _othersmusic 0.0))

(fn `UserConstructionScript`)