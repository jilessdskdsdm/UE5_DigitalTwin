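; BP_HighlightObject toggles a custom-depth highlight on tagged static mesh actors when the 1 key is pressed.
; A FlipFlop feeds SetHighlightTarget, which gets actors tagged "ta" through SetTagActorShow and switches their custom depth rendering and stencil value.
; It also switches Brightness and Saturation in the Mat_Highligt parameter collection, presumably driving a stencil-based post-process material.
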(event `self.ReceiveBeginPlay`
  (`self.EnableInput` (`GameplayStatics.GetPlayerController` 0)))

(event `Key|One`
  (params (Key :type "Key Structure"))
  (:`Pressed`
    (bind _isa (`/Engine/EditorBlueprintResources/StandardMacros.FlipFlop`)
      (:`A`
        _)
      (:`B`
        _))
    (`/DigitalTwin/Data/FL_FunctionLibrary.SetHighlightTarget` "ta" _isa)))

(event `SetHighlightTarget`
  (params (TagName :type Name) (bIsShow :type Boolean))
  (bind _tagactors (`FunctionLibrary.SetTagActorShow` TagName bIsShow))
  (for _array_element _tagactors
    (bind `_as静态网格体actor` (cast `StaticMeshActor` _array_element))
    (`/Engine/EditorBlueprintResources/StandardMacros.IsValid` `_as静态网格体actor`
      (:`Is Valid`
        (bind _staticmeshcomponent (`StaticMeshActor.StaticMeshComponent` `_as静态网格体actor`))
        (`PrimitiveComponent.SetRenderCustomDepth` _staticmeshcomponent bIsShow)
        (`PrimitiveComponent.SetCustomDepthStencilValue` _staticmeshcomponent (select `bool` bIsShow :`true` 1))
        (`KismetMaterialLibrary.SetScalarParameterValue` "/DigitalTwin/Material/Highlight/Mat_Highligt.Mat_Highligt" "Brightness" (select `bool` bIsShow :`false` 1.0 :`true` 0.35 :!type "Float (single-precision)"))
        (`KismetMaterialLibrary.SetScalarParameterValue` "/DigitalTwin/Material/Highlight/Mat_Highligt.Mat_Highligt" "Saturation" (select `bool` bIsShow :`true` 1.0 :!type "Float (single-precision)"))))))

(fn `UserConstructionScript`)