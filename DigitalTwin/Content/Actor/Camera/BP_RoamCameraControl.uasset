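; BP_RoamCameraControl is a manager that records and restores the starting transforms of every BP_RoamCamera in the level.
; On BeginPlay it gathers all roam camera actors and caches their transforms in an array parallel to the actor array.
; The InitialRoamCamera event resets each camera to its cached transform by matching index, without sweep or teleport.
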(event `self.ReceiveBeginPlay`
  (bind _outactors (`GameplayStatics.GetAllActorsOfClass` "/DigitalTwin/Actor/Camera/BP_RoamCamera.BP_RoamCamera_C"))
  (bind _output_get (set `self.AllRoamCamera` _outactors))
  (if (`KismetArrayLibrary.Array_IsNotEmpty` _output_get)
    (for _array_element (`self.AllRoamCamera`)
      (`KismetArrayLibrary.Array_Add` (`self.RC_InitialPosition`) (`self.GetTransform` _array_element)))))

(event `InitialRoamCamera`
  (for (_array_element _array_index) (`self.AllRoamCamera`)
    (`self.K2_SetActorTransform` _array_element (`|GetArrayItem` (`self.RC_InitialPosition`) _array_index) false false)))

(fn `UserConstructionScript`)