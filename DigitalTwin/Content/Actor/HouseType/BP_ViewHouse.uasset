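; House-viewing actor that slides a selected housing unit out from its house button and frames it with the camera.
; BeginPlay sets Roaming and Scenery tags and starts a Timeline lerp, with direction and height depending on building and floor.
; Camera input stays disabled during the move, then the house-type UI appears.
; SwitchCameraYHYJ opens a per-building floor-view widget; teardown hides the UI, restores input or unloads a streamed level.
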(event `ClickRoaming`)

(event `SwitchCameraYHYJ`
  (params (CameraIndex :type Integer))
  (bind ((`Building` _building)) (break `HouseData` (`self.HouseData`)))
  ; 切换相机到指定楼层
  (`FunctionLibrary.SwitchPawnControl` "Camera" CameraIndex)
  (bind _outcamera (`FunctionLibrary.SwitchCamera` CameraIndex))
  (bind _returnvalue (`|CreateWidget` "/Game/JL/BP/WBP_YHYJ.WBP_YHYJ_C" null (select `int` _building :`0` 0 :`1` 17 :`2` 16 :`3` 16 :`4` 9 :`5` 10 :`6` 10 :`7` 10 :`8` 16 :`9` 0 :`10` 0) (`self.Layer`) CameraIndex false 1 (select `int` _building :`0` 7425.0 :`1` 7425.0 :`2` 7425.0 :`3` 7045.0 :`4` 7145.0 :`5` 6605.0 :`6` 6585.0 :`7` 6675.0 :`8` 7005.0)))
  (bind _output_get (set `/DigitalTwin/UserWidget/WBP_MainMenu.CurrentScreen` _returnvalue (`/DigitalTwin/Data/FL_FunctionLibrary.GetMainMenu`)))
  (`UserWidget.AddToViewport` _output_get 0))

(event `ClickScenery`
  (params (YHYJCameraIndex :type Integer)))

(event `StartMove`
  (params (HouseButtonLocation :type "Vector Structure") (MoveDistance :type "Float (double-precision)" :default 1000.0) (MoveHeight :type "Float (double-precision)") (MoveDirection :type Boolean))
  ; 点击移动
  (`|ExecutionSequence`
    (:`then_0`
      (set `self.InitialLocation` (0.0 0.0 0.0))
      (set `self.EndLocation` (0.0 0.0 0.0)))
    (:`then_1`
      (set `self.InitialLocation` HouseButtonLocation)
      (set `self.EndLocation` (select `bool` MoveDirection :`false` (`KismetMathLibrary.MakeVector` (+ (.x (`self.InitialLocation`)) -500.0) (+ (.y (`self.InitialLocation`)) MoveDistance) (+ (.z (`self.InitialLocation`)) MoveHeight)) :`true` (`KismetMathLibrary.MakeVector` (+ (.x (`self.InitialLocation`)) MoveDistance) (+ (.y (`self.InitialLocation`)) -500.0) (+ (.z (`self.InitialLocation`)) MoveHeight)))))
    (:`then_2`
      (bind (_direction `_新建轨道_0`) (`Timeline|时间轴` :!via `PlayFromStart`)
        (:`Update`
          (`self.K2_SetActorLocation` (`KismetMathLibrary.VLerp` (`self.InitialLocation`) (`self.EndLocation`) `_新建轨道_0`))
          (`self.DisableInput` (`FunctionLibrary.GetCamera`) (`GameplayStatics.GetPlayerController` 0)))
        (:`Finished`
          (`|ExecutionSequence`
            (:`then_0`
              (bind _asbp_tag (cast `/DigitalTwin/Actor/Tag/BP_Tag` (`ChildActorComponent.ChildActor` (`self.Scenery`))))
              (`/Engine/EditorBlueprintResources/StandardMacros.IsValid` _asbp_tag
                (:`Is Valid`
                  (set `Tag.TagInfo` (make `TagInfo`) _asbp_tag))))
            (:`then_1`
              (bind _asbp_tag_2 (cast `/DigitalTwin/Actor/Tag/BP_Tag` (`ChildActorComponent.ChildActor` (`self.Roaming`))))
              (`/Engine/EditorBlueprintResources/StandardMacros.IsValid` _asbp_tag_2
                (:`Is Valid`
                  (set `Tag.TagInfo` (make `TagInfo`) _asbp_tag_2))))
            (:`then_2`
              (`/DigitalTwin/UserWidget/WBP_MainMenu.ShowHousType` (`/DigitalTwin/Data/FL_FunctionLibrary.GetMainMenu`) true (`.Building` (break `HouseData` (`self.HouseData`))))
              (`self.EnableInput` (`FunctionLibrary.GetCamera`) (`GameplayStatics.GetPlayerController` 0)))))))))

(event `falseDestroy`
  (`self.K2_DestroyActor`)
  (`GameplayStatics.UnloadStreamLevelBySoftObjectPtr` "/Game/Maps/03_ZhuAn/03_ZhuAnZhiWu_003.03_ZhuAnZhiWu_003"))

(event `self.ReceiveEndPlay`
  (params (EndPlayReason :type "EEndPlayReason Enum" :default "Destroyed"))
  (bind _mainmenu (`/DigitalTwin/Data/FL_FunctionLibrary.GetMainMenu`))
  (bind _returnvalue (`FunctionLibrary.GetCamera`))
  (`|ExecutionSequence`
    (:`then_0`
      (`/Engine/EditorBlueprintResources/StandardMacros.IsValid` _mainmenu
        (:`Is Valid`
          (`/DigitalTwin/UserWidget/WBP_MainMenu.ShowHousType` _mainmenu false 0))))
    (:`then_1`
      (`self.K2_DestroyActor`))
    (:`then_2`
      (`/Engine/EditorBlueprintResources/StandardMacros.IsValid` _returnvalue
        (:`Is Valid`
          (`self.EnableInput` _returnvalue (`GameplayStatics.GetPlayerController` 0)))))))

(event `self.ReceiveBeginPlay`
  (bind (_returnvalue_roll _returnvalue_pitch _returnvalue_yaw) (`KismetMathLibrary.BreakRotator` (`self.K2_GetActorRotation`)))
  (bind (_returnvalue_roll_2 _returnvalue_pitch_2 _returnvalue_yaw_2) (`KismetMathLibrary.BreakRotator` (`self.K2_GetActorRotation`)))
  (`|ExecutionSequence`
    (:`then_0`
      (`/DigitalTwin/Data/FL_FunctionLibrary.SetShowTag` "Roaming" true 0.25)
      (`/DigitalTwin/Data/FL_FunctionLibrary.SetShowTag` "Scenery" true 0.25))
    (:`then_1`
      (if (!= (`.Building` (break `HouseData` (`self.HouseData`))) 7)
        (`self.StartMove` (`self.K2_GetActorLocation` (`self.HouseButton`)) (`self.Move Distance`) (select `bool` (<= (`.Layer` (break `HouseData` (`self.HouseData`))) 3) :`true` 1500.0) true)
        (`FunctionLibrary.SwitchCameraLocation` 999 (`self.EndLocation`) (+ _returnvalue_yaw_2 -90.0))
        (else
          (`self.StartMove` (`self.K2_GetActorLocation` (`self.HouseButton`)) (* (`self.Move Distance`) -1.0) (select `bool` (<= (`.Layer` (break `HouseData` (`self.HouseData`))) 3) :`true` 1500.0))
          (`FunctionLibrary.SwitchCameraLocation` 998 (`self.EndLocation`) (+ _returnvalue_yaw -90.0)))))
    (:`then_2`
      (`SceneComponent.K2_SetRelativeLocation` (`self.Scenery`) (0.0 555.0 90.0) false false)
      (`SceneComponent.K2_SetRelativeLocation` (`self.Roaming`) (0.0 -200.0 90.0) false false))))

(fn `UserConstructionScript`)