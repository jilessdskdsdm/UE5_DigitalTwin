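; House button controller that spawns the buttons for every BP_HouseButton in the level and controls which building's buttons are shown.
; On BeginPlay it calls SpawnHouseButton on each one, picking floor count by building and a uniform vertical spacing, then hides all buttons.
; SetButtonVisual disables all buttons, then activates or deactivates those of the given building number.
; An older per-floor BP_Tag show/hide loop remains in that function, disconnected.
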(event `self.ReceiveBeginPlay`
  (`|ExecutionSequence`
    (:`then_0`
      (bind _outactors (`GameplayStatics.GetAllActorsOfClass` "/DigitalTwin/Actor/HouseType/BP_HouseButton.BP_HouseButton_C"))
      (for _array_element _outactors
        (`/Engine/EditorBlueprintResources/StandardMacros.IsValid` _array_element
          (:`Is Valid`
            (bind ((`Building` _building)) (break `HouseData` (`HouseButton.HouseData` _array_element)))
            (`HouseButton.SpawnHouseButton` _array_element (select `int` _building :`0` 300.0 :`1` 300.0 :`2` 300.0 :`3` 300.0 :`4` 300.0 :`5` 300.0 :`6` 300.0 :`7` 300.0 :`8` 300.0 :!type "Float (single-precision)") (select `int` _building :`0` 15.0 :`1` 16.0 :`2` 15.0 :`3` 15.0 :`4` 8.0 :`5` 9.0 :`6` 9.0 :`7` 9.0 :`8` 15.0 :!type "Float (single-precision)"))))))
    (:`then_1`
      (`self.DisableAllButtons`)
      (`self.SetButtonVisual` false))))

(fn `SetButtonVisual`
  (params (bIsShow :type Boolean) (ThatBuilding :type Integer))
  (locals (HButton :type "HouseButton Object Reference"))
  (`self.DisableAllButtons`)
  (`self.ActivateCurrentBuildingButton` ThatBuilding bIsShow))

(fn `UserConstructionScript`)