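; BP_HouseButton is a clickable room-unit button in a building showcase that previews the selected house.
; Hovering shows a widget with building number, room number and a floor area chosen by building.
; The bound house-click event destroys the clicked button's existing view house, spawns an odd or even BP_ViewHouse variant from the house data, and hides "loulou"-tagged actors.
; It also sets the main menu's return target; mesh clicks themselves only play a sound.
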(event `self.ReceiveBeginPlay`
  (add `self.OnHouseButtonClicked` (`|CreateDelegate` :!event `OnHouseButtonClickEvent`))
  (bind _widget (`self.Widget`)
    (:`then`
      (`SceneComponent.SetVisibility` _widget false false))
    (:`else`)))

(event `DestroyViewHouse`
  (bind _clickbutton (`self.ClickButton`)
    (:`then`
      (bind _viewhouse (`HouseButton.ViewHouse` _clickbutton)
        (:`then`
          (bind _asbp_view_house (cast `/DigitalTwin/Actor/HouseType/BP_ViewHouse` _viewhouse))
          (`self.K2_DestroyActor` _asbp_view_house)
          (set `HouseButton.ViewHouse` null _clickbutton))
        (:`else`)))
    (:`else`)))

(event `OnHouseButtonClickEvent` :!signature `self.OnHouseButtonClicked`
  (params (Button :type "HouseButton Object Reference") (Data :type "HouseData Structure (by ref)"))
  (set `self.ClickButton` Button)
  (set `/DigitalTwin/UserWidget/WBP_MainMenu.ReturnTargetName` "选中房" (`/DigitalTwin/Data/FL_FunctionLibrary.GetMainMenu`))
  (`|ExecutionSequence`
    (:`then_0`
      (`self.DestroyViewHouse`))
    (:`then_1`
      (bind _asbp_view_house (castclass `/DigitalTwin/Actor/HouseType/BP_ViewHouse` (`self.SpawnTarget` Data)))
      (bind _returnvalue (`|SpawnActorFromClass` _asbp_view_house (`KismetMathLibrary.MakeTransform` (.location (`self.GetTransform`)) (.rotation (`self.GetTransform`)) (0.8 0.8 1.0)) "Undefined" "MultiplyWithRoot" null 600.0 (`.Layer` (break `HouseData` Data)) -2300.0 (`self.ClickButton`) Data null))
      (set `self.ViewHouse` _returnvalue)
      (`FunctionLibrary.SetTagActorShow` "loulou"))))

(event `self.ButtonMesh.OnBeginCursorOver`
  (params (TouchedComponent :type "PrimitiveComponent Object Reference"))
  (bind (_roomnumber _building) (break `HouseData` (`self.HouseData`)))
  (bind _returnvalue (`GameplayStatics.GetActorOfClass` "/DigitalTwin/Actor/HouseType/BP_HouseButtonController.BP_HouseButtonController_C"))
  (for _array_element (`HouseButtonControl.GetAllHouseButton` _returnvalue)
    (if (== _array_element self)
      (bind _asbp_house_button (cast `/Game/Actor/HouseType/BP_HouseButton` _array_element))
      (bind _widget (`/Game/Actor/HouseType/BP_HouseButton.Widget` _asbp_house_button)
        (:`then`
          (bind _aswbp_no_click_tag (cast `/DigitalTwin/Actor/Tag/WBP_NoClickTag` (`WidgetComponent.GetWidget` _widget)))
          (`SceneComponent.SetVisibility` _widget true false)
          (`/DigitalTwin/Actor/Tag/WBP_NoClickTag.Satr` _aswbp_no_click_tag (`KismetTextLibrary.Conv_StringToText` (`KismetStringLibrary.Concat_StrStr` (`KismetStringLibrary.Conv_IntToString` _building) "#")) (`KismetTextLibrary.Conv_StringToText` _roomnumber) (select `int` _building :`0` "" :`1` "138㎡" :`2` "138㎡" :`3` "127㎡" :`4` "117㎡" :`5` "110㎡" :`6` "110㎡" :`7` "109㎡" :`8` "127㎡" :!type "Text")))
        (:`else`)))))

(event `VisD`
  (for _array_element (`SceneComponent.GetChildrenComponents` (`self.ButtonMesh`) false)
    (for _array_element_2 (`ActorComponent.ComponentTags` _array_element)
      (if (== _array_element_2 "ding")
        (`SceneComponent.SetVisibility` _array_element false true)))))

(event `self.ButtonMesh.OnEndCursorOver`
  (params (TouchedComponent :type "PrimitiveComponent Object Reference"))
  (bind _widget (`self.Widget`)
    (:`then`
      (`SceneComponent.SetVisibility` _widget false false))
    (:`else`)))

(event `self.ButtonMesh.OnClicked`
  (params (TouchedComponent :type "PrimitiveComponent Object Reference") (ButtonPressed :type "Key Structure"))
  (`/DigitalTwin/Data/FL_FunctionLibrary.PlayOthersMusic` "/DigitalTwin/Asset/Audio/YM-鼠标.YM-鼠标"))

(fn `SpawnTarget`
  (params (HouseData :type "HouseData Structure (by ref)"))
  (returns (ReturnValue :type "Object Class Reference"))
  (bind ((`OddOrEven` _oddoreven) (`Odd_SpawnViewHouse` _odd_spawnviewhouse) (`Even_SpawnViewHouse` _even_spawnviewhouse)) (break `HouseData` HouseData))
  (return (select `bool` _oddoreven :`false` _odd_spawnviewhouse :`true` _even_spawnviewhouse :!type "Object Class Reference")))

(fn `UserConstructionScript`)